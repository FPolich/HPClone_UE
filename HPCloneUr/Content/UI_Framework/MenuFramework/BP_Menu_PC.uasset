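; BP_Menu_PC is the main menu player controller that opens the gameplay level when Play is pressed.
; On BeginPlay it sets UI-only input, shows the cursor and defers setup to the next tick.
; That setup gets the BP_Menu_HUD and binds its menu widget's play-button event to load ThirdPersonMap by object reference.
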(event Custom|OpenLevelGame
  (Game|OpenLevel(byObjectReference) "/Game/ThirdPerson/Maps/ThirdPersonMap.ThirdPersonMap"))

(event Custom|Init
  (bind _asbp_menu_hud (Utilities|Casting|CastToBP_Menu_HUD (HUD|GetHUD)))
  (bind _output_get (Variables|Default|SetMenuHUDRef _asbp_menu_hud))
  (EventDispatchers|BindEventtoOnPlayButtonPress (Variables|/Game/UI_Framework/MenuFramework/BP_Menu_HUD.BP_Menu_HUD_C|GetMenuRef _output_get) (delegate Custom|OpenLevelGame)))

(event EventBeginPlay
  (Class|KismetSystemLibrary|SetTimerforNextTickDelegate (delegate Custom|Init))
  (Input|SetInputModeUIOnly self 0 "DoNotLock" false)
  (Variables|Default|SetbShowMouseCursor true))

(fn ConstructionScript)