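; BP_HarryPotterPC is a player controller that links the player character's health to the HUD health bar.
; On BeginPlay it caches the BP_HUD and the controlled BP_ThirdPersonCharacter, binds to the character health component's change event, then sets game-only input with a hidden cursor.
; Each health change sends current over max health to the HUD's health bar update.
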(event EventBeginPlay
  (bind _asbp_hud (Utilities|Casting|CastToBP_HUD (HUD|GetHUD)))
  (Variables|Default|SetHUDRef _asbp_hud)
  (bind _asbp_third_person_character (Utilities|Casting|CastToBP_ThirdPersonCharacter (Pawn|GetControlledPawn)))
  (bind _output_get (Variables|Default|SetPlayerRef _asbp_third_person_character))
  (EventDispatchers|BindEventtoOnHealthChanged (Variables|/Game/ThirdPerson/Blueprints/BP_ThirdPersonCharacter.BP_ThirdPersonCharacter_C|GetAC_HealthComponent _output_get) (EventDispatchers|CreateEvent :!event OnHealthChanged))
  (Input|SetInputModeGameOnly self false)
  (Variables|Default|SetbShowMouseCursor false))

(fn ConstructionScript)

(fn OnHealthChanged
  (params (CurrentHealth :type Float%20%28double-precision%29) (MaxHealth :type Float%20%28double-precision%29))
  (Default|UpdateHealthBar (Variables|Default|GetHUDRef) (/ CurrentHealth MaxHealth)))