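; Health component that tracks an actor's current and maximum health.
; On BeginPlay it fills health to the maximum, and damage and healing functions adjust it within zero and that maximum.
; Every change broadcasts OnHealthChanged with current and maximum values.
; ReduceHealth also broadcasts OnDeath whenever health is at zero afterwards, with no guard against repeat calls.
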(event EventBeginPlay
  (CallFunction|Initialize))

(event EventTick
  (params (DeltaSeconds :type Float%20%28single-precision%29)))

(fn Initialize
  (Variables|Default|SetCurrentHealth (Variables|Default|GetMaxHealth))
  (CallFunction|HealthChanged))

(fn ReduceHealth
  (params (DamageAmount :type Float%20%28double-precision%29))
  (bind _output_get (Variables|Default|SetCurrentHealth (Math|Float|Clamp(Float) (- (Variables|Default|GetCurrentHealth) DamageAmount) 0.0 (Variables|Default|GetMaxHealth))))
  (CallFunction|HealthChanged)
  (if (<= _output_get 0.0)
    (Default|CallOnDeath)))

(fn AddHealth
  (params (HealingAmount :type Float%20%28double-precision%29))
  (Variables|Default|SetCurrentHealth (Math|Float|Clamp(Float) (+ HealingAmount (Variables|Default|GetCurrentHealth)) 0.0 (Variables|Default|GetMaxHealth)))
  (CallFunction|HealthChanged))

(fn HealthChanged
  (Default|CallOnHealthChanged (Variables|Default|GetCurrentHealth) (Variables|Default|GetMaxHealth)))